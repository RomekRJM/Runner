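; Trigger box Blueprint that turns a group of overlapping actors a quarter turn, apparently one face of a Rubik's-style cube, using a hard-coded "F" move.
; The move string gives a pivot actor tag and direction, with an apostrophe or B/L face each flipping the sign.
; Each Tick attaches overlapping actors to the tagged pivot and pitches it until accumulated rotation reaches 90 degrees, without clamping overshoot.
; The detach function is an unused stub.
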(event Collision|EventActorBeginOverlap
  (params (OtherActor :type Actor%20Object%20Reference)))

(event EventTick
  (params (DeltaSeconds :type Float%20%28single-precision%29))
  (bind (_clockwise _rotation) (CallFunction|GetRotationInstructions "F"))
  (if (Math|Boolean|Equal(Boolean) (Variables|Default|GetRotationFinished) false)
    (bind _found (CallFunction|GetFirstOverlapingActorwithTag _rotation))
    (if (Utilities|IsValid _found)
      (CallFunction|AttachOverlapingActorsto _found)
      (Transformation|AddActorLocalRotation _found (* (Math|Rotator|MakeRotator 0.0 (* _clockwise (Variables|Default|GetRotationSpeed)) 0.0) DeltaSeconds) false false)
      (bind _output_get (Variables|Default|SetRotatedSoFar (+ (Math|Float|Absolute(Float) (.Pitch (Math|Rotator|BreakRotator (* (Math|Rotator|MakeRotator 0.0 (* _clockwise (Variables|Default|GetRotationSpeed)) 0.0) DeltaSeconds)))) (Variables|Default|GetRotatedSoFar))))
      (Variables|Default|SetRotationFinished (>= _output_get 9e+01)))))

(fn ConstructionScript)

(fn AttachOverlapingActorsto
  (params (ParentActor :type Actor%20Object%20Reference))
  (for _array_element (Collision|GetOverlappingActors 0 :!class /Script/Engine.Actor)
    (if (!= _array_element ParentActor)
      (Transformation|AttachActorToActor _array_element ParentActor "None" "KeepWorld" "KeepWorld" "KeepRelative" true))))

(fn DettachActorsfrom
  (params (ParentActor :type Actor%20Object%20Reference) (Actors :type Array%20of%20Actor%20Object%20References))
  (for _array_element Actors
    (if (!= _array_element ParentActor)
      _)))

(fn GetFirstOverlapingActorwithTag
  (params (Tag :type Name))
  (bind _outactors (Actor|GetAllActorswithTag Tag))
  (for _array_element _outactors
    (if (> (Utilities|Array|FindItem (Collision|GetOverlappingActors 0 :!class /Script/Engine.Actor) _array_element) -1)
      (return _array_element)))
  (return 0))

(fn GetRotationInstructions
  (params (Move :type String))
  (bind _returnvalue (Utilities|String|GetSubstring Move 0))
  (if (Utilities|String|Contains Move "'")
    (Variables|Default|SetCWise -1.0)
    (else
      (Variables|Default|SetCWise 1.0)))
  (if (or (Utilities|Enum|Equal(Enum) _returnvalue "B") (Utilities|Enum|Equal(Enum) _returnvalue "L"))
    (Variables|Default|SetCWise (* (Variables|Default|GetCWise) -1.0)))
  (return (Variables|Default|GetCWise) (Utilities|String|StringToName _returnvalue)))