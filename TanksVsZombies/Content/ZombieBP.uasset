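; Paper2D zombie actor Blueprint that handles the green zombie's walk, attack and death visuals through flipbooks.
; Walk events scale playback rate with movement speed between walk and run, while attack events restart a one-shot animation.
; Death disables tick, lowers the actor and shows the dead flipbook while a timeline drives sprite color alpha, then destroys it.
; Crushed deaths also run a second timeline that animates the flipbook's scale.
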(event EventBeginPlay)

(event Collision|EventActorBeginOverlap
  (params (OtherActor :type Actor%20Object%20Reference)))

(event EventZombieDie
  (params (DamageType :type EDamageType%20Enum))
  (bind _self self)
  (bind _paperflipbook (Variables|Default|GetPaperFlipbook))
  (Actor|Tick|SetActorTickEnabled _self)
  (Transformation|SetActorLocation (+ (Transformation|GetActorLocation) "0, 0,-10.000000") false false)
  (Class|TankStatics|PlayFlipbook _paperflipbook "/Game/Sprites/GreenZombie/GreenZombieDead.GreenZombieDead" false 1.0 false)
  (Utilities|FlowControl|Sequence
    (:then_0
      (bind _newtrack_0 (Timeline|Timeline_0 PlayFromStart)
        (:Update
          (Sprite|SetSpriteColor _paperflipbook (Utilities|Struct|MakeLinearColor 0.0 0.0 0.0 _newtrack_0)))
        (:Finished
          (Actor|DestroyActor _self))))
    (:then_1
      (switch Utilities|FlowControl|Switch|SwitchonEDamageType DamageType
        (:Crushed
          (bind _newtrack_2 (Timeline|Timeline_1 Play)
            (:Update
              (Transformation|SetWorldScale3D _paperflipbook (Math|Conversions|ToVector(Float) _newtrack_2)))))))))

(event EventTick
  (params (DeltaSeconds :type Float%20%28single-precision%29)))

(event EventZombieWalk
  (params (DeltaSeconds :type Float%20%28single-precision%29) (DistanceWalkedThisFrame :type Vector))
  (Class|TankStatics|PlayFlipbook (Variables|Default|GetPaperFlipbook) "/Game/Sprites/GreenZombie/GreenZombieWalk.GreenZombieWalk" true (Math|Float|MapRangeClamped (/ (Math|Vector|VectorLength DistanceWalkedThisFrame) DeltaSeconds) (Variables|Default|GetWalkSpeed) (Variables|Default|GetRunSpeed) 1.0 2.0) false))

(event EventZombieAttack
  (params (DeltaSeconds :type Float%20%28single-precision%29))
  (bind _paperflipbook (Variables|Default|GetPaperFlipbook))
  (Sprite|SetFlipbook _paperflipbook "/Game/Sprites/GreenZombie/GreenZombieAttack.GreenZombieAttack")
  (Components|Timeline|SetLooping _paperflipbook false)
  (Audio|Components|Audio|Play _paperflipbook)
  (Components|Timeline|PlayfromStart _paperflipbook)
  (Components|Timeline|SetPlayRate _paperflipbook 1.0))

(fn ConstructionScript)